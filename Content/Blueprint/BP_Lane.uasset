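; BP_Lane is a traffic lane actor that spawns BP_Vehicle actors from either side and removes itself when the player overlaps DestroyLaneZone.
; A looping timer spawns a vehicle at the left or right spawn point at random, only while the previous one is no longer valid.
; Each vehicle receives a travel direction, with right-side spawns rotated 180 degrees.
; Two DestroyVehicle trigger volumes destroy overlapping vehicles, freeing the lane for the next spawn.
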(event `self.ReceiveBeginPlay`
  (`KismetSystemLibrary.K2_SetTimer` null "SpawnVehicleRandom" 0.5 true))

(event `self.DestroyLaneZone.OnComponentBeginOverlap`
  (params (OverlappedComponent :type "PrimitiveComponent Object Reference") (OtherActor :type "Actor Object Reference") (OtherComp :type "PrimitiveComponent Object Reference") (OtherBodyIndex :type Integer) (bFromSweep :type Boolean) (SweepResult :type "HitResult Structure (by ref)"))
  (cast `/Game/Blueprint/BP_Player` OtherActor)
  (`self.K2_DestroyActor` self))

(event `self.DestroyVehicle1.OnComponentBeginOverlap`
  (params (OverlappedComponent :type "PrimitiveComponent Object Reference") (OtherActor :type "Actor Object Reference") (OtherComp :type "PrimitiveComponent Object Reference") (OtherBodyIndex :type Integer) (bFromSweep :type Boolean) (SweepResult :type "HitResult Structure (by ref)"))
  (bind _asbp_vehicle (cast `/Game/Blueprint/BP_Vehicle` OtherActor))
  (`self.K2_DestroyActor` _asbp_vehicle))

(event `self.DestroyVehicle.OnComponentBeginOverlap`
  (params (OverlappedComponent :type "PrimitiveComponent Object Reference") (OtherActor :type "Actor Object Reference") (OtherComp :type "PrimitiveComponent Object Reference") (OtherBodyIndex :type Integer) (bFromSweep :type Boolean) (SweepResult :type "HitResult Structure (by ref)"))
  (bind _asbp_vehicle (cast `/Game/Blueprint/BP_Vehicle` OtherActor))
  (`self.K2_DestroyActor` _asbp_vehicle))

(fn `RotateVehicle`
  (`self.K2_SetActorRelativeRotation` (`self.NewestVehicle`) (struct :`Yaw` 180.0) false false))

(fn `SpawnVehicle`
  (params (Location :type "Vector Structure") (Direction :type "Float (double-precision)"))
  (bind _returnvalue (`|SpawnActorFromClass` "/Game/Blueprint/BP_Vehicle.BP_Vehicle_C" (`KismetMathLibrary.MakeTransform` Location (`KismetMathLibrary.MakeRotator` 0.0)) "Undefined" "OverrideRootScale" null null))
  (bind _output_get (set `self.NewestVehicle` _returnvalue))
  (set `/Game/Blueprint/BP_Vehicle.Direction` Direction _output_get)
  (set `/Game/Blueprint/BP_Vehicle.DefaultDirection` Direction _output_get))

(fn `SpawnVehicleRandom`
  (`/Engine/EditorBlueprintResources/StandardMacros.IsValid` (`self.NewestVehicle`)
    (:`Is Not Valid`
      (switch `int` (`KismetMathLibrary.RandomIntegerInRange` 0 1)
        (:`Default`
          (`self.SpawnVehicle` (`SceneComponent.K2_GetComponentLocation` (`self.RightSpawn`)) -1.0)
          (`self.RotateVehicle`))
        (:`0`
          (`self.SpawnVehicle` (`SceneComponent.K2_GetComponentLocation` (`self.LeftSpawn`)) 1.0))))))

(fn `UserConstructionScript`)