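; BP_GrassSpawner builds a chain of BP_Starting_Grass lanes, laying 30 at BeginPlay from a fixed offset to the player pawn.
; Each new piece becomes NewestGrass, whose scene components position the next one.
; SpawnGrassAtTrigger extends the chain from the trigger spawn point, using a counter to add extra X offset on every fifth call.
; A separate SpawnRandom function spawns and tracks BP_RandomLane, though nothing here calls it.
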(event `self.ReceiveBeginPlay`
  (`self.SpawnInitialGrass`))

(fn `SpawnGrass`
  (params (`Grass Location` :type "Vector Structure"))
  (bind _returnvalue (`|SpawnActorFromClass` "/Game/Blueprint/BP_Starting_Grass.BP_Starting_Grass_C" (`KismetMathLibrary.MakeTransform` `Grass Location`) "Undefined" "OverrideRootScale" null null))
  (bind _output_get (set `self.Newest Grass` _returnvalue))
  (set `/Game/Blueprint/BP_Starting_Grass.LaneSpawner` null self _output_get))

(fn `SpawnGrassAtSpawnPoint`
  (`self.SpawnGrass` (`SceneComponent.K2_GetComponentLocation` (`/Game/Blueprint/BP_Starting_Grass.NewLaneSpawn` (`self.Newest Grass`)))))

(fn `SpawnGrassAtTrigger`
  (switch `int` (mod (`self.GrassCounter`) 5)
    (:`Default`
      (`self.SpawnGrass` (`SceneComponent.K2_GetComponentLocation` (`/Game/Blueprint/BP_Starting_Grass.GrassPlayerTriggerSpawnPoint` (`self.Newest Grass`))))
      (set `self.GrassCounter` (+ (`self.GrassCounter`) 1)))
    (:`0`
      (`self.SpawnGrass` (+ (`SceneComponent.K2_GetComponentLocation` (`/Game/Blueprint/BP_Starting_Grass.GrassPlayerTriggerSpawnPoint` (`self.Newest Grass`))) (180.0 0.0 0.0)))
      (set `self.GrassCounter` (+ (`self.GrassCounter`) 1)))))

(fn `SpawnInitialGrass`
  (for _ (range 30)
    (`/Engine/EditorBlueprintResources/StandardMacros.IsValid` (`self.Newest Grass`)
      (:`Is Valid`
        (`self.SpawnGrassAtSpawnPoint`))
      (:`Is Not Valid`
        (`self.SpawnGrass` (+ (`self.K2_GetActorLocation` (`GameplayStatics.GetPlayerPawn` 0)) (-2700.0 0.0 -80.0)))))))

(fn `SpawnRandom`
  (params (Location :type "Vector Structure"))
  (bind _returnvalue (`|SpawnActorFromClass` "/Game/Blueprint/BP_RandomLane.BP_RandomLane_C" (`KismetMathLibrary.MakeTransform` Location) "Undefined" "OverrideRootScale" null null))
  (set `self.NewestRandomLane` _returnvalue))

(fn `UserConstructionScript`)