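; BP_Log is a log actor that slides along the world Y axis each Tick at MaxSpeed times Direction, using swept movement.
; Its Safety volume sets OnLog on an overlapping BP_Player and clears it on exit.
; Its MoveZone volume toggles CanMovePlayer, but the logic that would move the player's mesh with the log is disconnected and never runs.
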(event `self.ReceiveTick`
  (params (DeltaSeconds :type "Float (single-precision)"))
  (`self.K2_AddActorWorldOffset` (`KismetMathLibrary.MakeVector` 0.0 (* DeltaSeconds (* (`self.MaxSpeed`) (`self.Direction`)))) true))

(event `self.Safety.OnComponentBeginOverlap`
  (params (OverlappedComponent :type "PrimitiveComponent Object Reference") (OtherActor :type "Actor Object Reference") (OtherComp :type "PrimitiveComponent Object Reference") (OtherBodyIndex :type Integer) (bFromSweep :type Boolean) (SweepResult :type "HitResult Structure (by ref)"))
  (bind _asbp_player (cast `/Game/Blueprint/BP_Player` OtherActor))
  (set `/Game/Blueprint/BP_Player.onLog` true _asbp_player))

(event `self.Safety.OnComponentEndOverlap`
  (params (OverlappedComponent :type "PrimitiveComponent Object Reference") (OtherActor :type "Actor Object Reference") (OtherComp :type "PrimitiveComponent Object Reference") (OtherBodyIndex :type Integer))
  (bind _asbp_player (cast `/Game/Blueprint/BP_Player` OtherActor))
  (set `/Game/Blueprint/BP_Player.onLog` false _asbp_player))

(event `self.MoveZone.OnComponentBeginOverlap`
  (params (OverlappedComponent :type "PrimitiveComponent Object Reference") (OtherActor :type "Actor Object Reference") (OtherComp :type "PrimitiveComponent Object Reference") (OtherBodyIndex :type Integer) (bFromSweep :type Boolean) (SweepResult :type "HitResult Structure (by ref)"))
  (cast `/Game/Blueprint/BP_Player` OtherActor)
  (set `self.CanMovePlayer` true))

(event `self.MoveZone.OnComponentEndOverlap`
  (params (OverlappedComponent :type "PrimitiveComponent Object Reference") (OtherActor :type "Actor Object Reference") (OtherComp :type "PrimitiveComponent Object Reference") (OtherBodyIndex :type Integer))
  (cast `/Game/Blueprint/BP_Player` OtherActor)
  (set `self.CanMovePlayer` false))

(fn `UserConstructionScript`)