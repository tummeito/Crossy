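; Player Blueprint for a hop-across-traffic game, moving a mesh in four directions and dying when a vehicle overlaps its Kill component.
; Each input turns the mesh and chains HopBegin and HopEnd offsets through MoveComponentTo for an up-then-down arc, with the camera following only forward and back.
; LeftSpeedUp and RightSpeedUp triggers override overlapping vehicles' speed and direction, restoring defaults on exit.
; Once dead, Tick reveals an Eagle and moves it to the player.
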(event `InputAction|MoveForward`
  (params (Key :type "Key Structure"))
  (bind _maxspeed (`self.MaxSpeed`))
  (bind _maxspeed_2 (`self.MaxSpeed`))
  (:`Pressed`
    (`self.HopBegin` (`KismetMathLibrary.MakeVector` _maxspeed))
    (`self.MoveCamera` (`KismetMathLibrary.MakeVector` _maxspeed))
    (bind _output_get (set `self.MeshRotation` (`self.DefaultRotation`)))
    (`KismetSystemLibrary.MoveComponentTo` (`self.StaticMesh`) (`self.HopPosition`) _output_get false false 0.2)
    (`self.HopEnd` (`KismetMathLibrary.MakeVector` _maxspeed_2))
    (`self.MoveCamera` (`KismetMathLibrary.MakeVector` _maxspeed_2))
    (`KismetSystemLibrary.MoveComponentTo` (`self.StaticMesh`) (`self.HopPosition`) _output_get false false 0.2)
    (`SceneComponent.K2_AddRelativeLocation` (`self.LeftSpeedUp`) (`KismetMathLibrary.MakeVector` (* (`self.MaxSpeed`) 2.0)) true false)
    (`SceneComponent.K2_AddRelativeLocation` (`self.RightSpeedUp`) (`KismetMathLibrary.MakeVector` (* (`self.MaxSpeed`) 2.0)) true false)
    (`KismetSystemLibrary.MoveComponentTo` (`self.Camera`) (`self.CamPosition`) (`SceneComponent.RelativeRotation` (`self.Camera`)) false false 0.4)))

(event `self.ReceiveBeginPlay`
  (bind _output_get (set `self.DefaultRotation` (`SceneComponent.RelativeRotation` (`self.StaticMesh`))))
  (set `self.MeshRotation` _output_get)
  (set `self.CamPosition` (`SceneComponent.RelativeLocation` (`self.Camera`)))
  (set `self.HopPosition` (`SceneComponent.RelativeLocation` (`self.StaticMesh`))))

(event `self.ReceiveTick`
  (params (DeltaSeconds :type "Float (single-precision)"))
  (bind _eagle (`self.Eagle`))
  (if (`self.isDead`)
    (`SceneComponent.SetVisibility` _eagle true false)
    (`KismetSystemLibrary.MoveComponentTo` _eagle (`SceneComponent.RelativeLocation` (`self.StaticMesh`)) (`SceneComponent.RelativeRotation` _eagle) false false 0.1)))

(event `InputAction|MoveBack`
  (params (Key :type "Key Structure"))
  (bind (_defaultrotation_roll _defaultrotation_pitch _defaultrotation_yaw) (`KismetMathLibrary.BreakRotator` (`self.DefaultRotation`)))
  (bind _returnvalue (* (`self.MaxSpeed`) -1.0))
  (bind _returnvalue_2 (* (`self.MaxSpeed`) -1.0))
  (:`Pressed`
    (`self.HopBegin` (`KismetMathLibrary.MakeVector` _returnvalue))
    (`self.MoveCamera` (`KismetMathLibrary.MakeVector` _returnvalue))
    (bind _output_get (set `self.MeshRotation` (`KismetMathLibrary.MakeRotator` _defaultrotation_roll _defaultrotation_pitch (+ _defaultrotation_yaw 180.0))))
    (`KismetSystemLibrary.MoveComponentTo` (`self.StaticMesh`) (`self.HopPosition`) _output_get)
    (`self.HopEnd` (`KismetMathLibrary.MakeVector` _returnvalue_2))
    (`self.MoveCamera` (`KismetMathLibrary.MakeVector` _returnvalue_2))
    (`KismetSystemLibrary.MoveComponentTo` (`self.StaticMesh`) (`self.HopPosition`) _output_get)
    (`SceneComponent.K2_AddRelativeLocation` (`self.LeftSpeedUp`) (`KismetMathLibrary.MakeVector` (* _returnvalue_2 2.0)) true false)
    (`SceneComponent.K2_AddRelativeLocation` (`self.RightSpeedUp`) (`KismetMathLibrary.MakeVector` (* _returnvalue_2 2.0)) true false)
    (`KismetSystemLibrary.MoveComponentTo` (`self.Camera`) (`self.CamPosition`) (`SceneComponent.RelativeRotation` (`self.Camera`)) false false 0.4)))

(event `self.LeftSpeedUp.OnComponentBeginOverlap`
  (params (OverlappedComponent :type "PrimitiveComponent Object Reference") (OtherActor :type "Actor Object Reference") (OtherComp :type "PrimitiveComponent Object Reference") (OtherBodyIndex :type Integer) (bFromSweep :type Boolean) (SweepResult :type "HitResult Structure (by ref)"))
  (bind _asbp_vehicle (cast `/Game/Blueprint/BP_Vehicle` OtherActor))
  (set `/Game/Blueprint/BP_Vehicle.MaxSpeed` 750.0 _asbp_vehicle)
  (set `/Game/Blueprint/BP_Vehicle.Direction` 1.0 _asbp_vehicle))

(event `self.LeftSpeedUp.OnComponentEndOverlap`
  (params (OverlappedComponent :type "PrimitiveComponent Object Reference") (OtherActor :type "Actor Object Reference") (OtherComp :type "PrimitiveComponent Object Reference") (OtherBodyIndex :type Integer))
  (bind _asbp_vehicle (cast `/Game/Blueprint/BP_Vehicle` OtherActor))
  (set `/Game/Blueprint/BP_Vehicle.MaxSpeed` (`/Game/Blueprint/BP_Vehicle.DefaultSpeed` _asbp_vehicle) _asbp_vehicle)
  (set `/Game/Blueprint/BP_Vehicle.Direction` (`/Game/Blueprint/BP_Vehicle.DefaultDirection` _asbp_vehicle) _asbp_vehicle))

(event `InputAction|MoveRight`
  (params (Key :type "Key Structure"))
  (bind _maxspeed (`self.MaxSpeed`))
  (bind (_defaultrotation_roll _defaultrotation_pitch _defaultrotation_yaw) (`KismetMathLibrary.BreakRotator` (`self.DefaultRotation`)))
  (:`Pressed`
    (`self.HopBegin` (`KismetMathLibrary.MakeVector` 0.0 _maxspeed))
    (bind _output_get (set `self.MeshRotation` (`KismetMathLibrary.MakeRotator` _defaultrotation_roll _defaultrotation_pitch (+ _defaultrotation_yaw 90.0))))
    (`KismetSystemLibrary.MoveComponentTo` (`self.StaticMesh`) (`self.HopPosition`) _output_get)
    (`self.HopEnd` (`KismetMathLibrary.MakeVector` 0.0 _maxspeed))
    (`KismetSystemLibrary.MoveComponentTo` (`self.StaticMesh`) (`self.HopPosition`) _output_get)
    (`SceneComponent.K2_SetRelativeLocation` (`self.LeftSpeedUp`) (`KismetMathLibrary.MakeVector` 0.0 (* _maxspeed 2.0)) false false)
    (`SceneComponent.K2_SetRelativeLocation` (`self.RightSpeedUp`) (`KismetMathLibrary.MakeVector` 0.0 (* _maxspeed 2.0)) false false)
    (`KismetSystemLibrary.MoveComponentTo` (`self.Camera`) (`self.CamPosition`) (`SceneComponent.RelativeRotation` (`self.Camera`)) false false 0.4)))

(event `self.RightSpeedUp.OnComponentBeginOverlap`
  (params (OverlappedComponent :type "PrimitiveComponent Object Reference") (OtherActor :type "Actor Object Reference") (OtherComp :type "PrimitiveComponent Object Reference") (OtherBodyIndex :type Integer) (bFromSweep :type Boolean) (SweepResult :type "HitResult Structure (by ref)"))
  (bind _asbp_vehicle (cast `/Game/Blueprint/BP_Vehicle` OtherActor))
  (set `/Game/Blueprint/BP_Vehicle.MaxSpeed` 750.0 _asbp_vehicle)
  (set `/Game/Blueprint/BP_Vehicle.Direction` -1.0 _asbp_vehicle))

(event `self.RightSpeedUp.OnComponentEndOverlap`
  (params (OverlappedComponent :type "PrimitiveComponent Object Reference") (OtherActor :type "Actor Object Reference") (OtherComp :type "PrimitiveComponent Object Reference") (OtherBodyIndex :type Integer))
  (bind _asbp_vehicle (cast `/Game/Blueprint/BP_Vehicle` OtherActor))
  (set `/Game/Blueprint/BP_Vehicle.MaxSpeed` (`/Game/Blueprint/BP_Vehicle.DefaultSpeed` _asbp_vehicle) _asbp_vehicle)
  (set `/Game/Blueprint/BP_Vehicle.Direction` (`/Game/Blueprint/BP_Vehicle.DefaultDirection` _asbp_vehicle) _asbp_vehicle))

(event `InputAction|MoveLeft`
  (params (Key :type "Key Structure"))
  (bind (_defaultrotation_roll _defaultrotation_pitch _defaultrotation_yaw) (`KismetMathLibrary.BreakRotator` (`self.DefaultRotation`)))
  (bind _returnvalue (* (`self.MaxSpeed`) -1.0))
  (:`Pressed`
    (`self.HopBegin` (`KismetMathLibrary.MakeVector` 0.0 _returnvalue))
    (bind _output_get (set `self.MeshRotation` (`KismetMathLibrary.MakeRotator` _defaultrotation_roll _defaultrotation_pitch (+ _defaultrotation_yaw -90.0))))
    (`KismetSystemLibrary.MoveComponentTo` (`self.StaticMesh`) (`self.HopPosition`) _output_get)
    (`self.HopEnd` (`KismetMathLibrary.MakeVector` 0.0 _returnvalue))
    (`KismetSystemLibrary.MoveComponentTo` (`self.StaticMesh`) (`self.HopPosition`) _output_get)
    (`SceneComponent.K2_SetRelativeLocation` (`self.LeftSpeedUp`) (`KismetMathLibrary.MakeVector` 0.0 (* _returnvalue 2.0)) false false)
    (`SceneComponent.K2_SetRelativeLocation` (`self.RightSpeedUp`) (`KismetMathLibrary.MakeVector` 0.0 (* _returnvalue 2.0)) false false)
    (`KismetSystemLibrary.MoveComponentTo` (`self.Camera`) (`self.CamPosition`) (`SceneComponent.RelativeRotation` (`self.Camera`)) false false 0.4)))

(event `self.Kill.OnComponentBeginOverlap`
  (params (OverlappedComponent :type "PrimitiveComponent Object Reference") (OtherActor :type "Actor Object Reference") (OtherComp :type "PrimitiveComponent Object Reference") (OtherBodyIndex :type Integer) (bFromSweep :type Boolean) (SweepResult :type "HitResult Structure (by ref)"))
  (cast `/Game/Blueprint/BP_Vehicle` OtherActor)
  (set `self.isDead` true))

(fn `HopBegin`
  (params (Direction :type "Vector Structure"))
  (if (`self.CanHop`)
    (set `self.HopPosition` (+ (+ Direction (`self.HopPosition`)) (0.0 0.0 90.0)))))

(fn `HopEnd`
  (params (Direction :type "Vector Structure"))
  (if (`self.CanHop`)
    (set `self.HopPosition` (+ (+ Direction (`self.HopPosition`)) (0.0 0.0 -90.0)))))

(fn `MoveCamera`
  (params (Direction :type "Vector Structure"))
  (set `self.CamPosition` (+ Direction (`self.CamPosition`))))

(fn `QuitGame`
  (`KismetSystemLibrary.QuitGame` null "Quit"))

(fn `ResetHop`
  (params (Direction :type "Vector Structure"))
  (set `self.CanHop` true))

(fn `UserConstructionScript`)