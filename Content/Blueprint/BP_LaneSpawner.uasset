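; BP_LaneSpawner builds the chain of lanes in the level, laying an opening run of grass lanes at BeginPlay from an offset to the player pawn.
; Each lane spawns at the newest lane's NextSpawn point, with BP_RandomLane's child actor either set to grass or randomized.
; Lanes receive a spawner reference; random-lane and separate BP_Lane spawn functions are defined but not called here.
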(event `self.ReceiveBeginPlay`
  (`self.SpawnInitialGrassLane`))

(fn `SpawnGrassLane`
  (params (SpawnLocation :type "Vector Structure"))
  (bind _returnvalue (`|SpawnActorFromClass` "/Game/Blueprint/BP_RandomLane.BP_RandomLane_C" (`KismetMathLibrary.MakeTransform` SpawnLocation) "Undefined" "OverrideRootScale" null null))
  (bind _output_get (set `self.NewestRandomLane` _returnvalue))
  (`ChildActorComponent.SetChildActorClass` (`/Game/Blueprint/BP_RandomLane.ChildActor` _output_get) (`/Game/Blueprint/BP_RandomLane.Grass` _output_get))
  (set `/Game/Blueprint/BP_RandomLane.LaneSpawner` self _output_get))

(fn `SpawnGrassLaneAtSpawnPoint`
  (`self.SpawnGrassLane` (`SceneComponent.K2_GetComponentLocation` (`/Game/Blueprint/BP_RandomLane.NextSpawn` (`self.NewestRandomLane`)))))

(fn `SpawnInitialGrassLane`
  (for _ (range 30)
    (`/Engine/EditorBlueprintResources/StandardMacros.IsValid` (`self.NewestRandomLane`)
      (:`Is Valid`
        (`self.SpawnGrassLaneAtSpawnPoint`))
      (:`Is Not Valid`
        (`self.SpawnGrassLane` (+ (`self.K2_GetActorLocation` (`GameplayStatics.GetPlayerPawn` 0)) (-2700.0 0.0 -80.0)))))))

(fn `SpawnLane`
  (params (SpawnLocation :type "Vector Structure"))
  (bind _returnvalue (`|SpawnActorFromClass` "/Game/Blueprint/BP_Lane.BP_Lane_C" (`KismetMathLibrary.MakeTransform` SpawnLocation) "Undefined" "OverrideRootScale" null null))
  (bind _output_get (set `self.Newest Lane` _returnvalue))
  (set `/Game/Blueprint/BP_Lane.LaneSpawner` self _output_get))

(fn `SpawnLaneAtSpawnPoint`
  (`self.SpawnLane` (`SceneComponent.K2_GetComponentLocation` (`/Game/Blueprint/BP_Lane.NewLaneSpawn` (`self.Newest Lane`)))))

(fn `SpawnRandomLane`
  (params (SpawnLocation :type "Vector Structure"))
  (bind _returnvalue (`|SpawnActorFromClass` "/Game/Blueprint/BP_RandomLane.BP_RandomLane_C" (`KismetMathLibrary.MakeTransform` SpawnLocation) "Undefined" "OverrideRootScale" null null))
  (bind _output_get (set `self.NewestRandomLane` _returnvalue))
  (`/Game/Blueprint/BP_RandomLane.RandomizeChildActor` _output_get)
  (set `/Game/Blueprint/BP_RandomLane.LaneSpawner` self _output_get))

(fn `SpawnRandomLaneAtSpawnPoint`
  (`self.SpawnRandomLane` (`SceneComponent.K2_GetComponentLocation` (`/Game/Blueprint/BP_RandomLane.NextSpawn` (`self.NewestRandomLane`)))))

(fn `SpawnRandomLaneAtTrigger`
  (`self.SpawnRandomLane` (`SceneComponent.K2_GetComponentLocation` (`/Game/Blueprint/BP_RandomLane.NextSpawn` (`self.NewestRandomLane`)))))

(fn `UserConstructionScript`)