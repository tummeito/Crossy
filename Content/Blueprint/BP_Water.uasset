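; BP_Water is a water lane that sends floating logs across and kills a player who enters without being on one.
; A looping timer spawns a BP_Log at a random side, heading in the matching direction, whenever the previous log is no longer valid.
; Two DestroyLog volumes remove logs, the Kill volume sets IsDead on the player, and DestroyLaneZone destroys the lane when the player overlaps it.
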(event `self.ReceiveBeginPlay`
  (`KismetSystemLibrary.K2_SetTimer` null "SpawnLogRandom" 0.5 true))

(event `self.DestroyLaneZone.OnComponentBeginOverlap`
  (params (OverlappedComponent :type "PrimitiveComponent Object Reference") (OtherActor :type "Actor Object Reference") (OtherComp :type "PrimitiveComponent Object Reference") (OtherBodyIndex :type Integer) (bFromSweep :type Boolean) (SweepResult :type "HitResult Structure (by ref)"))
  (cast `/Game/Blueprint/BP_Player` OtherActor)
  (`self.K2_DestroyActor` self))

(event `self.DestroyLog.OnComponentBeginOverlap`
  (params (OverlappedComponent :type "PrimitiveComponent Object Reference") (OtherActor :type "Actor Object Reference") (OtherComp :type "PrimitiveComponent Object Reference") (OtherBodyIndex :type Integer) (bFromSweep :type Boolean) (SweepResult :type "HitResult Structure (by ref)"))
  (bind _asbp_log (cast `/Game/Blueprint/BP_Log` OtherActor))
  (`self.K2_DestroyActor` _asbp_log))

(event `self.DestroyLog1.OnComponentBeginOverlap`
  (params (OverlappedComponent :type "PrimitiveComponent Object Reference") (OtherActor :type "Actor Object Reference") (OtherComp :type "PrimitiveComponent Object Reference") (OtherBodyIndex :type Integer) (bFromSweep :type Boolean) (SweepResult :type "HitResult Structure (by ref)"))
  (bind _asbp_log (cast `/Game/Blueprint/BP_Log` OtherActor))
  (`self.K2_DestroyActor` _asbp_log))

(event `self.Kill.OnComponentBeginOverlap`
  (params (OverlappedComponent :type "PrimitiveComponent Object Reference") (OtherActor :type "Actor Object Reference") (OtherComp :type "PrimitiveComponent Object Reference") (OtherBodyIndex :type Integer) (bFromSweep :type Boolean) (SweepResult :type "HitResult Structure (by ref)"))
  (bind _asbp_player (cast `/Game/Blueprint/BP_Player` OtherActor))
  (if (not (`/Game/Blueprint/BP_Player.onLog` _asbp_player))
    (set `/Game/Blueprint/BP_Player.isDead` true _asbp_player)))

(fn `SpawnLog`
  (params (Location :type "Vector Structure") (Direction :type "Float (double-precision)"))
  (bind _returnvalue (`|SpawnActorFromClass` "/Game/Blueprint/BP_Log.BP_Log_C" (`KismetMathLibrary.MakeTransform` Location) "Undefined" "OverrideRootScale" null null))
  (bind _output_get (set `self.NewestLog` _returnvalue))
  (set `/Game/Blueprint/BP_Log.Direction` Direction _output_get))

(fn `SpawnLogRandom`
  (`/Engine/EditorBlueprintResources/StandardMacros.IsValid` (`self.NewestLog`)
    (:`Is Not Valid`
      (switch `int` (`KismetMathLibrary.RandomIntegerInRange` 0 1)
        (:`0`
          (`self.SpawnLog` (`SceneComponent.K2_GetComponentLocation` (`self.LeftSpawn`)) 1.0))
        (:`1`
          (`self.SpawnLog` (`SceneComponent.K2_GetComponentLocation` (`self.RightSpawn`)) -1.0))))))

(fn `UserConstructionScript`)