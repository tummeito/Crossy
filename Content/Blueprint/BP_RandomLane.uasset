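; BP_RandomLane is a lane segment that randomly becomes a Lane, Grass, Water or Railroad child actor on BeginPlay.
; BeginPlay also loads any saved high score onto BP_Player.
; When the player overlaps NextLaneSpawnZone, it adds a point, asks LaneSpawner to spawn another lane and destroys the zone.
; A score matching or beating the high score is written to the SaveGame_HS slot, creating the save if missing.
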(event `self.ReceiveBeginPlay`
  (`self.RandomizeChildActor`)
  (`GameplayStatics.DoesSaveGameExist` (`self.Slot Name`))
  (if true
    (bind _returnvalue (`GameplayStatics.LoadGameFromSlot` (`self.Slot Name`)))
    (bind _output_get (set `self.SaveSubclass` _returnvalue))
    (bind _assave_game_hs (cast `/Game/Blueprint/SaveGame_HS` _output_get))
    (bind _asbp_player (cast `/Game/Blueprint/BP_Player` (`GameplayStatics.GetPlayerPawn` 0)))
    (set `/Game/Blueprint/BP_Player.Highscore` (`/Game/Blueprint/SaveGame_HS.Highscore` _assave_game_hs) _asbp_player)))

(event `self.NextLaneSpawnZone.OnComponentBeginOverlap`
  (params (OverlappedComponent :type "PrimitiveComponent Object Reference") (OtherActor :type "Actor Object Reference") (OtherComp :type "PrimitiveComponent Object Reference") (OtherBodyIndex :type Integer) (bFromSweep :type Boolean) (SweepResult :type "HitResult Structure (by ref)"))
  (bind _asbp_player (cast `/Game/Blueprint/BP_Player` OtherActor))
  (bind _score (`/Game/Blueprint/BP_Player.Score` _asbp_player))
  (set `/Game/Blueprint/BP_Player.Score` (+ _score 1.0) _asbp_player)
  (`/Game/Blueprint/BP_LaneSpawner.SpawnRandomLaneAtTrigger` (`self.LaneSpawner`))
  (`ActorComponent.K2_DestroyComponent` (`self.NextLaneSpawnZone`))
  (if (>= _score (`/Game/Blueprint/BP_Player.Highscore` _asbp_player))
    (bind _output_get (set `/Game/Blueprint/BP_Player.Highscore` _score _asbp_player))
    (bind _returnvalue (`GameplayStatics.DoesSaveGameExist` (`self.Slot Name`)))
    (if _returnvalue
      (bind _returnvalue_2 (`GameplayStatics.LoadGameFromSlot` (`self.Slot Name`)))
      (bind _output_get_2 (set `self.SaveSubclass` _returnvalue_2))
      (bind _assave_game_hs (cast `/Game/Blueprint/SaveGame_HS` _output_get_2))
      (set `/Game/Blueprint/SaveGame_HS.Highscore` _output_get _assave_game_hs)
      (`GameplayStatics.SaveGameToSlot` (`self.SaveSubclass`) (`self.Slot Name`))
      (else
        (bind _returnvalue_3 (`GameplayStatics.CreateSaveGameObject` "/Game/Blueprint/SaveGame_HS.SaveGame_HS_C"))
        (bind _output_get_3 (set `self.SaveSubclass` _returnvalue_3))
        (bind _assave_game_hs_2 (cast `/Game/Blueprint/SaveGame_HS` _output_get_3))
        (set `/Game/Blueprint/SaveGame_HS.Highscore` _output_get _assave_game_hs_2)
        (`GameplayStatics.SaveGameToSlot` (`self.SaveSubclass`) (`self.Slot Name`))))))

(fn `RandomizeChildActor`
  (`ChildActorComponent.SetChildActorClass` (`self.ChildActor`) (select `int` (`KismetMathLibrary.RandomIntegerInRange` 0 3) :`0` (`self.Lane`) :`1` (`self.Grass`) :`2` (`self.Water`) :`3` (`self.Railroad`))))

(fn `UserConstructionScript`)