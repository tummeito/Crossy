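; HUD_HUD puts the Widget_HS widget on screen at BeginPlay and handles the game-over sequence.
; Every Tick it polls IsDead on the BP_Player pawn; when true it adds a Widget_GAMEOVER, disables player input and quits the game after a short delay.
; The death check has no one-shot guard, so a new game-over widget is created on each tick until the quit.
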(event `self.ReceiveBeginPlay`
  (bind _returnvalue (`|CreateWidget` "/Game/Blueprint/Widget_HS.Widget_HS_C" (`GameplayStatics.GetPlayerController` 0)))
  (`UserWidget.AddToViewport` _returnvalue 0))

(event `self.ReceiveTick`
  (params (DeltaSeconds :type "Float (single-precision)"))
  (bind _asbp_player (cast `/Game/Blueprint/BP_Player` (`GameplayStatics.GetPlayerPawn` 0)))
  (if (`/Game/Blueprint/BP_Player.isDead` _asbp_player)
    (bind _returnvalue (`|CreateWidget` "/Game/Blueprint/Widget_GAMEOVER.Widget_GAMEOVER_C" (`GameplayStatics.GetPlayerController` 0)))
    (`UserWidget.AddToViewport` _returnvalue 0)
    (bind _asbp_player_2 (cast `/Game/Blueprint/BP_Player` (`GameplayStatics.GetPlayerPawn` 0)))
    (`self.DisableInput` _asbp_player_2 (`GameplayStatics.GetPlayerController` 0))
    (`KismetSystemLibrary.Delay` 1.0)
    (`KismetSystemLibrary.QuitGame` null "Quit")))

(fn `UserConstructionScript`)